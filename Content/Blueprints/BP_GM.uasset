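; BP_GM populates the level with NPCs and fire spawns when play begins.
; SpawnNPC and SpawnFire loop over NPCCount and FireCount, picking random reachable navigation points within a fixed radius around a slightly raised world origin.
; Each successful query spawns an actor, adjusted for collision but always spawned; failed queries are skipped.
; NPCs use BP_NPC, while the fire spawn shows no actor class.
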(event `self.ReceiveBeginPlay`
  (`self.Spawn NPC` (`self.NPCCount`))
  (`self.Spawn Fire`))

(fn `Spawn Fire`
  (bind (_randomlocation _returnvalue) (`NavigationSystemV1.K2_GetRandomReachablePointInRadius` (0.0 0.0 100.0) 4000.0 null null))
  (for _ (range 1 (+ (`self.FireCount`) 1))
    (if _returnvalue
      (`|SpawnActorFromClass` "/Game/Blueprints/Props/BP_FireZone.BP_FireZone_C" (`KismetMathLibrary.MakeTransform` _randomlocation) "AdjustIfPossibleButAlwaysSpawn" "MultiplyWithRoot" null null))))

(fn `Spawn NPC`
  (params (NPCCount :type Integer))
  (bind (_randomlocation _returnvalue) (`NavigationSystemV1.K2_GetRandomReachablePointInRadius` (0.0 0.0 100.0) 4000.0 null null))
  (for _ (range 1 (+ NPCCount 1))
    (if _returnvalue
      (`|SpawnActorFromClass` "/Game/Blueprints/Character/NPC/BP_NPC.BP_NPC_C" (`KismetMathLibrary.MakeTransform` _randomlocation) "AdjustIfPossibleButAlwaysSpawn" "MultiplyWithRoot" null null))))

(fn `UserConstructionScript`)