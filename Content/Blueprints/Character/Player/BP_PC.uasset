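; Player controller that turns Enhanced Input actions into commands on the possessed BP_Player character.
; On BeginPlay it sets game-only input, caches the pawn as BP_Player and adds the IMC_Default mapping context.
; Movement follows control-rotation yaw, while crouch, jump, attack and sprint forward to the character's own functions.
; Started and Triggered share the same logic; Canceled and Completed release crouch, jump and sprint.
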(event `self.ReceiveBeginPlay`
  (bind _returnvalue (subsystem `EnhancedInputLocalPlayerSubsystem`))
  (`WidgetBlueprintLibrary.SetInputMode_GameOnly` self)
  (bind _asbp_player (cast `/Game/Blueprints/Character/Player/BP_Player` (`self.K2_GetPawn`)))
  (set `self.BP Player Ref` _asbp_player)
  (`/Engine/EditorBlueprintResources/StandardMacros.IsValid` _returnvalue
    (:`Is Valid`
      (`EnhancedInputSubsystemInterface.AddMappingContext` _returnvalue "/Game/Blueprints/Character/Player/Inputs/IMC_Default.IMC_Default" 0 (struct)))))

(event `EnhancedInput|/Game/Blueprints/Character/Player/Inputs/Actions/IA_Move`
  (params (ActionValue :type "Vector2D Structure") (ElapsedSeconds :type "Float (double-precision)") (TriggeredSeconds :type "Float (double-precision)") (InputAction :type "InputAction Object Reference" :default "/Game/Blueprints/Character/Player/Inputs/Actions/IA_Move.IA_Move"))
  (bind (_x _y) (`KismetMathLibrary.BreakVector2D` ActionValue))
  (bind (_returnvalue_roll _returnvalue_pitch _returnvalue_yaw) (`KismetMathLibrary.BreakRotator` (`self.GetControlRotation`)))
  (bind _bp_player_ref (`self.BP Player Ref`))
  (bind _returnvalue (`KismetMathLibrary.MakeRotator` 0.0 0.0 _returnvalue_yaw))
  (:`Triggered`
    (`|ExecutionSequence` :!label _label
      (:`then_0`
        (`Pawn.AddMovementInput` _bp_player_ref (`KismetMathLibrary.GetRightVector` _returnvalue) _x false))
      (:`then_1`
        (`Pawn.AddMovementInput` _bp_player_ref (`KismetMathLibrary.GetForwardVector` _returnvalue) _y false))))
  (:`Started`
    (goto _label)))

(event `EnhancedInput|/Game/Blueprints/Character/Player/Inputs/Actions/IA_Crouch`
  (params (ActionValue :type Boolean) (ElapsedSeconds :type "Float (double-precision)") (TriggeredSeconds :type "Float (double-precision)") (InputAction :type "InputAction Object Reference" :default "/Game/Blueprints/Character/Player/Inputs/Actions/IA_Crouch.IA_Crouch"))
  (bind _bp_player_ref (`self.BP Player Ref`))
  ; 이거 왜안될까?
  (:`Triggered`
    (`Character.Crouch` _bp_player_ref :!label _label_2))
  (:`Started`
    (goto _label_2))
  (:`Canceled`
    (`Character.UnCrouch` _bp_player_ref :!label _label_3))
  (:`Completed`
    (goto _label_3)))

(event `EnhancedInput|/Game/Blueprints/Character/Player/Inputs/Actions/IA_Jump`
  (params (ActionValue :type Boolean) (ElapsedSeconds :type "Float (double-precision)") (TriggeredSeconds :type "Float (double-precision)") (InputAction :type "InputAction Object Reference" :default "/Game/Blueprints/Character/Player/Inputs/Actions/IA_Jump.IA_Jump"))
  (bind _bp_player_ref (`self.BP Player Ref`))
  (:`Triggered`
    (`Character.Jump` _bp_player_ref :!label _label_4))
  (:`Started`
    (goto _label_4))
  (:`Canceled`
    (`Character.StopJumping` _bp_player_ref :!label _label_5))
  (:`Completed`
    (goto _label_5)))

(event `EnhancedInput|/Game/Blueprints/Character/Player/Inputs/Actions/IA_Attack`
  (params (ActionValue :type Boolean) (ElapsedSeconds :type "Float (double-precision)") (TriggeredSeconds :type "Float (double-precision)") (InputAction :type "InputAction Object Reference" :default "/Game/Blueprints/Character/Player/Inputs/Actions/IA_Attack.IA_Attack"))
  (:`Triggered`
    (`/Game/Blueprints/Character/Player/BP_Player.CallAttack` (`self.BP Player Ref`) :!label _label_6))
  (:`Started`
    (goto _label_6)))

(event `EnhancedInput|/Game/Blueprints/Character/Player/Inputs/Actions/IA_Sprint`
  (params (ActionValue :type Boolean) (ElapsedSeconds :type "Float (double-precision)") (TriggeredSeconds :type "Float (double-precision)") (InputAction :type "InputAction Object Reference" :default "/Game/Blueprints/Character/Player/Inputs/Actions/IA_Sprint.IA_Sprint"))
  (bind _bp_player_ref (`self.BP Player Ref`))
  (:`Triggered`
    (`/Game/Blueprints/Character/Player/BP_Player.CallSprint` _bp_player_ref true :!label _label_7))
  (:`Started`
    (goto _label_7))
  (:`Canceled`
    (`/Game/Blueprints/Character/Player/BP_Player.CallSprint` _bp_player_ref false :!label _label_8))
  (:`Completed`
    (goto _label_8)))

(fn `UserConstructionScript`)