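; BP_Player is the player character Blueprint, handling networked attack and sprint.
; Call events forward to client-to-server and server-to-multicast events (C2S/S2M naming) that play the attack montage or set max walk speed.
; Attacks only start from Idle or Move, then switch HumanState to AttackSkill.
; HP-bar and death logic is present but unconnected, and a helper returns the cast BP_PlayerState.
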(event `CallAttack`
  (switch `/Game/Blueprints/Character/Player/E_State` (`self.HumanState`)
    (:`NewEnumerator0`
      (`self.C2S_Attack`))))

(event `C2S_Attack`
  (switch `/Game/Blueprints/Character/Player/E_State` (`self.HumanState`)
    (:`NewEnumerator0`
      (`self.S2M_Attack`))))

(event `S2M_Attack`
  (set `self.HumanState` "NewEnumerator1")
  (`self.PlayAnimMontage` "/Game/Blueprints/Character/Animations/Attack/AM_Attack.AM_Attack"))

(event `CallSprint`
  (params (bIsSprint :type Boolean))
  (`self.C2S_Sprint` bIsSprint))

(event `C2S_Sprint`
  (params (bIsSprint :type Boolean))
  (set `self.bIsSprint` bIsSprint)
  (`self.CtoS_UpdateSpeed`))

(event `CtoS_UpdateSpeed`
  (if (`self.bIsSprint`)
    (`self.S2M_Sprint` (`self.GetSprintSpeed`))
    (else
      (`self.S2M_Sprint` (`self.WalkSpeed`)))))

(event `S2M_Sprint`
  (params (Speed :type "Float (double-precision)"))
  (set `CharacterMovementComponent.MaxWalkSpeed` Speed (`self.CharacterMovement`)))

(fn `GetPlayerState`
  (returns (PlayerState :type "/Game/Blueprints/Character/Player/BP_PlayerState Object Reference"))
  (bind _asbp_player_state (cast `/Game/Blueprints/Character/Player/BP_PlayerState` (`self.PlayerState`)))
  (`/Engine/EditorBlueprintResources/StandardMacros.IsValid` _asbp_player_state
    (:`Is Valid`
      (return _asbp_player_state))
    (:`Is Not Valid`
      (return null))))

(fn `GetSprintSpeed`
  (returns (Speed :type "Float (double-precision)"))
  (return (`self.SprintSpeed`)))

(fn `UserConstructionScript`
  (`parent.UserConstructionScript`))